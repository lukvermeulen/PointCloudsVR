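; Player character for flying through a point cloud scene in VR or desktop, with camera-relative movement and a stereo toggle.
; On BeginPlay it snaps tagged HUD and Collider actors onto the left and right motion controllers.
; Right-controller inputs slide and resize the collider, writing its radius to BPA_Collider.
; Widget interaction components emulate left clicks from mouse or grip, with a per-frame debug line trace as the laser pointer.
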(event EventBeginPlay
  (Utilities|FlowControl|Sequence
    (:then_0
      ;[1 1 1] attach HUD to motion controller and scale / rotate it correctly so it is visible
      (bind _outactors (Actor|GetAllActorswithTag "HUD"))
      (for _array_element _outactors
        (bind _output_get (Variables|Default|SetHUD (Variables|/Script/Engine.Actor|GetRootComponent _array_element)))
        (Transformation|AttachComponentToComponent _output_get (Variables|Default|GetL_MotionController) "None" "SnapToTarget" "SnapToTarget" "SnapToTarget" false)
        (Transformation|SetRelativeScale3D (Variables|Default|GetHUD) "0.150000,0.150000,0.150000")
        (Transformation|SetRelativeRotation (Variables|Default|GetHUD) "0,180.000000, 0" false false)))
    (:then_1
      ;[1 1 1] attach collider to motion controller and offset it by standard value
      (bind _outactors_2 (Actor|GetAllActorswithTag "Collider"))
      (for _array_element_2 _outactors_2
        (bind _output_get_2 (Variables|Default|SetCollider (Variables|/Script/Engine.Actor|GetRootComponent _array_element_2)))
        (Transformation|AttachComponentToComponent _output_get_2 (Variables|Default|GetR_MotionController) "None" "SnapToTarget" "SnapToTarget" "SnapToTarget" false)
        (Transformation|SetRelativeLocation (Variables|Default|GetCollider) "100.000000, 0, 0" false false)))))

(event EventTick
  (params (DeltaSeconds :type Float%20%28single-precision%29))
  (bind _r_motioncontroller (Variables|Default|GetR_MotionController))
  (bind _returnvalue (Transformation|GetWorldLocation _r_motioncontroller))
  ;[1 1 1] for laserbeam
  (Collision|LineTraceByChannel _returnvalue (+ _returnvalue (* (Math|Vector|GetForwardVector (Variables|Default|GetWidgetInteraction_VR)) (Variables|Default|GetLaserDistance))) "TraceTypeQuery1" false 0 "ForOneFrame"))

(event Input|ActionEvents|InputActionToggleVR
  (params (Key :type Key%20Structure))
  (:Pressed
    (Utilities|FlowControl|FlipFlop
      (:A
        (Development|ExecuteConsoleCommand "stereo on" 0))
      (:B
        (Development|ExecuteConsoleCommand "stereo off" 0)))))

(event Input|AxisEvents|InputAxisMoveForward
  (params (AxisValue :type Float%20%28single-precision%29))
  (bind _returnvalue (Game|GetPlayerCameraManager 0))
  (bind _returnvalue_2 (Transformation|GetActorForwardVector _returnvalue))
  (Pawn|Input|AddMovementInput (Math|Vector|MakeVector (.x _returnvalue_2) (.y _returnvalue_2) 0.0) AxisValue false))

(event Input|AxisEvents|InputAxisMoveUp
  (params (AxisValue :type Float%20%28single-precision%29))
  ;[1 1 1] Fly up and down
  (Pawn|Input|AddMovementInput "0, 0,1.000000" AxisValue false))

(event Input|AxisEvents|InputAxisMoveDown
  (params (AxisValue :type Float%20%28single-precision%29))
  ;[1 1 1] Fly up and down
  (Pawn|Input|AddMovementInput "0, 0,1.000000" AxisValue false))

(event Input|AxisEvents|InputAxisMoveRight
  (params (AxisValue :type Float%20%28single-precision%29))
  (bind _returnvalue (Game|GetPlayerCameraManager 0))
  (bind _returnvalue_2 (Transformation|GetActorRightVector _returnvalue))
  (Pawn|Input|AddMovementInput (Math|Vector|MakeVector (.x _returnvalue_2) (.y _returnvalue_2) 0.0) AxisValue false))

(event Input|KeyboardEvents|MotionControllerRightThumbstickY
  (params (AxisValue :type Float%20%28single-precision%29))
  (bind _collider (Variables|Default|GetCollider))
  ;[1 1 1] Move Collider away and towards hand
  (Transformation|SetRelativeLocation _collider (Math|Vector|MakeVector (+ (* AxisValue -1e+01) (.x (Variables|/Script/Engine.SceneComponent|GetRelativeLocation _collider))) 0.0 0.0) false false))

(event Input|MouseEvents|RightMouseButton
  (params (Key :type Key%20Structure))
  (bind _widgetinteraction (Variables|Default|GetWidgetInteraction))
  ;[1 1 1] widget interactions
  (:Pressed
    (Class|WidgetInteractionComponent|PressPointerKey _widgetinteraction "LeftMouseButton"))
  (:Released
    (Class|WidgetInteractionComponent|ReleasePointerKey _widgetinteraction "LeftMouseButton")))

(event Input|KeyboardEvents|MotionControllerRightFaceButton2
  (params (Key :type Key%20Structure))
  (bind _collider (Variables|Default|GetCollider))
  ;[1 1 1] make collider bigger
  (:Pressed
    (Transformation|SetRelativeScale3D _collider (+ (Variables|/Script/Engine.SceneComponent|GetRelativeScale3D _collider) (Variables|Default|GetColliderScaleIncrement)))
    ;[1 1 1] calculate the new collider radius from the scale and set new value
    (bind _outactors (Actor|GetAllActorswithTag "Collider"))
    (bind _asbpa_collider (Utilities|Casting|CastToBPA_Collider (Utilities|Array|Get(acopy) _outactors)))
    (bind _output_get (Variables|/Game/Collider/BPA_Collider.BPA_Collider_C|SetColliderRadius _asbpa_collider (Math|Float|Truncate (* (Class|KismetMathLibrary|GetMinElement (Variables|/Script/Engine.SceneComponent|GetRelativeScale3D (Variables|Default|GetCollider))) 5e+01))))
    (Development|PrintString (Utilities|String|ToString(Integer) _output_get))))

(event Input|KeyboardEvents|MotionControllerRightFaceButton1
  (params (Key :type Key%20Structure))
  (bind _colliderscaleincrement (Variables|Default|GetColliderScaleIncrement))
  (bind _collider (Variables|Default|GetCollider))
  (bind _relativescale3d (Variables|/Script/Engine.SceneComponent|GetRelativeScale3D _collider))
  ;[1 1 1] make collider smaller and chack that it does not get too small / negative
  (:Pressed
    (if (not (< (Class|KismetMathLibrary|GetMinElement _relativescale3d) _colliderscaleincrement))
      (Transformation|SetRelativeScale3D _collider (- _relativescale3d _colliderscaleincrement))
      ;[1 1 1] calculate the new collider radius from the scale and set new value
      (bind _outactors (Actor|GetAllActorswithTag "Collider"))
      (bind _asbpa_collider (Utilities|Casting|CastToBPA_Collider (Utilities|Array|Get(acopy) _outactors)))
      (bind _output_get (Variables|/Game/Collider/BPA_Collider.BPA_Collider_C|SetColliderRadius _asbpa_collider (Math|Float|Truncate (* (Class|KismetMathLibrary|GetMinElement (Variables|/Script/Engine.SceneComponent|GetRelativeScale3D (Variables|Default|GetCollider))) 5e+01))))
      (Development|PrintString (Utilities|String|ToString(Integer) _output_get)))))

(event Input|KeyboardEvents|MotionControllerRightGrip1
  (params (Key :type Key%20Structure))
  (bind _widgetinteraction_vr (Variables|Default|GetWidgetInteraction_VR))
  ;[1 1 1] widget interactions
  (:Pressed
    (Class|WidgetInteractionComponent|PressPointerKey _widgetinteraction_vr "LeftMouseButton"))
  (:Released
    (Class|WidgetInteractionComponent|ReleasePointerKey _widgetinteraction_vr "LeftMouseButton")))

(fn ConstructionScript)